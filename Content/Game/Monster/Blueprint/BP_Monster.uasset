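; BP_Monster is a monster pawn that roams by AI-moving to random reachable points around its current location.
; On BeginPlay it starts the loop unless targeting; each successful move leads to a timed pause, then another move, with IsMoving tracking the state.
; A failed move has no handler, so the loop stops there.
; Hearing a noise through PawnSensing only sets IsTargetting, which the running loop never rechecks.
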(event OnHearNoise(PawnSensing)
  (params (Instigator :type Pawn%20Object%20Reference) (Location :type Vector%20%28by%20ref%29 :default "0, 0, 0") (Volume :type Float%20%28single-precision%29))
  (Variables|Default|SetIs%20Targetting true))

(event Custom|Wait
  ;[0.05098 0.05098 0.05098] Pause time of Monster
  (Variables|Default|SetIsMoving false)
  (Utilities|FlowControl|Delay 4.0)
  (CallFunction|RestartMoving))

(event Custom|Restart%20moving
  ;[0.05098 0.05098 0.05098] Base state of monster
  (AI|AIMoveTo self (.RandomLocation (AI|Navigation|GetRandomReachablePointinRadius (Transformation|GetActorLocation) 1.5e+03 0 0)) 0 5.0 false
    (:then
      (Variables|Default|SetIsMoving true))
    (:OnSuccess
      (CallFunction|Wait))))

(event EventBeginPlay
  ;[0.05098 0.05098 0.05098] Base state of monster
  (if (not (Variables|Default|GetIs%20Targetting))
    (AI|AIMoveTo self (.RandomLocation (AI|Navigation|GetRandomReachablePointinRadius (Transformation|GetActorLocation) 1.5e+03 0 0)) 0 5.0 false
      (:then
        (Variables|Default|SetIsMoving true))
      (:OnSuccess
        (CallFunction|Wait)))))

(fn ConstructionScript)