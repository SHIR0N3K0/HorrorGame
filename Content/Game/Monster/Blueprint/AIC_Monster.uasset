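; AI controller for the monster that runs BT_Monster and feeds it what the monster perceives.
; While IsTargeting is false, perception updates pass to separate sight and hearing handlers that write to the blackboard.
; Sight tracks only the player, setting or clearing TargetActor and saving LastKnownLocation when seen.
; Hearing stores the stimulus location from any source as TargetLocation.
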(event OnTargetPerceptionUpdated(AIPerception)
  (params (Actor :type Actor%20Object%20Reference) (Stimulus :type AI%20Stimulus%20Structure))
  ;[0.05098 0.05098 0.05098] Sense
  (if (not (Variables|Default|GetIsTargeting?))
    (CallFunction|SightSense Actor Stimulus)
    (CallFunction|HearingSense Stimulus Actor)))

(event EventBeginPlay
  ;[0.05098 0.05098 0.05098] Run behavior + REF
  (Utilities|FlowControl|Sequence
    (:then_0
      (bind _asbp_player (Utilities|Casting|CastToBP_Player (Game|Player|GetPlayerPawn 0)))
      (Variables|Default|SetAs%20BP%20Player _asbp_player))
    (:then_1
      (AI|RunBehaviorTree "/Game/Game/Monster/Blueprint/BT_Monster.BT_Monster"))))

(fn ConstructionScript)

(fn SightSense
  (params (Actor :type Actor%20Object%20Reference) (Stimulus :type AI%20Stimulus%20Structure))
  (bind _returnvalue (Class|AIPerceptionSystem|GetSenseClassforStimulus Stimulus))
  (if (== _returnvalue "/Script/AIModule.AISense_Sight")
    (if (== Actor (Game|GetPlayerCharacter 0))
      (AI|Components|Blackboard|SetValueasObject (AI|GetBlackboard 0) (Variables|Default|GetTargetActor) (Utilities|SelectObject (Game|GetPlayerCharacter 0) 0 (.bsuccessfullysensed Stimulus)))
      (if (.bsuccessfullysensed Stimulus)
        (AI|Components|Blackboard|SetValueasVector (AI|GetBlackboard 0) (Variables|Default|GetLastKnownLocation) (.stimuluslocation Stimulus)))
      (else
        (return)))
    (else
      (return))))

(fn HearingSense
  (params (Stimulus :type AI%20Stimulus%20Structure) (Actor :type Actor%20Object%20Reference))
  (bind _returnvalue (Class|AIPerceptionSystem|GetSenseClassforStimulus Stimulus))
  (if (== _returnvalue "/Script/AIModule.AISense_Hearing")
    (AI|Components|Blackboard|SetValueasVector (AI|GetBlackboard 0) (Variables|Default|GetTargetLocation) (.StimulusLocation (Utilities|Struct|BreakAIStimulus Stimulus)))
    (else
      (return))))