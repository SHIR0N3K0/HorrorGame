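; BP_note is an interactable note that opens a reading screen when the player interacts with it.
; On BeginPlay it caches a reference to the BP_Player pawn.
; The Aimed event sets that player's focus enum.
; Interact pauses the game, adds a WBP_note widget to the viewport, shows the mouse cursor and switches input to UI-only focused on the widget.
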(event EventAimed
  (Variables|/Game/Game/Character/Blueprint/BP_Player.BP_Player_C|SetEnum%20Focus%20REF (Variables|REF|GetPlayer%20REF) "NewEnumerator0"))

(event EventBeginPlay
  (bind _asbp_player (Utilities|Casting|CastToBP_Player (Game|Player|GetPlayerPawn 0)))
  (Variables|REF|SetPlayer%20REF _asbp_player))

(event EventInteract
  (bind _returnvalue (Game|GetPlayerController 0))
  (Game|SetGamePaused true)
  (bind _returnvalue_2 (UserInterface|CreateWidget "/Game/Game/Blueprint/widget/WBP_note.WBP_note_C"))
  (UserInterface|Viewport|AddtoViewport _returnvalue_2 0)
  (Variables|/Script/Engine.PlayerController|SetbShowMouseCursor _returnvalue true)
  (Input|SetInputModeUIOnly _returnvalue _returnvalue_2 "DoNotLock" false))

(fn ConstructionScript)