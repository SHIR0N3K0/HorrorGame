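; BP_medal_door is an interactable door that opens only when the player carries the medallion, which it consumes.
; When aimed at, it sets the player's focus enum to one of two states, depending on whether the medallion is held.
; On interact with the medallion, it plays a stone door sound and a timeline shifts the mesh vertically by a Move offset, clearing the medallion as it updates.
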(event EventAimed
  (Variables|/Game/Game/Character/Blueprint/BP_Player.BP_Player_C|SetEnum%20Focus%20REF (Variables|REF|GetPlayer%20REF) "NewEnumerator1")
  (if (== (Variables|/Game/Game/Character/Blueprint/BP_Player.BP_Player_C|GetMedaillon (Variables|REF|GetPlayer%20REF)) 1)
    (Variables|/Game/Game/Character/Blueprint/BP_Player.BP_Player_C|SetEnum%20Focus%20REF (Variables|REF|GetPlayer%20REF) "NewEnumerator2")))

(event EventBeginPlay
  (bind _asbp_player (Utilities|Casting|CastToBP_Player (Game|Player|GetPlayerPawn 0)))
  (Variables|REF|SetPlayer%20REF _asbp_player))

(event EventInteract
  (bind _staticmesh1 (Variables|Default|GetStaticMesh1))
  (bind _relativelocation (Variables|/Script/Engine.SceneComponent|GetRelativeLocation _staticmesh1))
  (if (== (Variables|/Game/Game/Character/Blueprint/BP_Player.BP_Player_C|GetMedaillon (Variables|REF|GetPlayer%20REF)) 1)
    (Audio|PlaySound2D "/Game/Game/Sound/stone_door.stone_door" 1.0 1.0 0.0 0 0)
    (Variables|Default|Setstart (.z (Variables|/Script/Engine.SceneComponent|GetRelativeLocation (Variables|Default|GetStaticMesh1))))
    (bind _newtrack_0 (Timeline|Timeline Play)
      (:Update
        (Transformation|SetRelativeLocation (Variables|Default|GetStaticMesh1) (Math|Vector|MakeVector (.x _relativelocation) (.y _relativelocation) (+ (Variables|Default|Getstart) (* _newtrack_0 (Variables|Default|Getmove)))) false false)
        (Variables|/Game/Game/Character/Blueprint/BP_Player.BP_Player_C|SetMedaillon (Variables|REF|GetPlayer%20REF) 0)))))

(fn ConstructionScript)