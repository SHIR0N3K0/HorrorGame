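; BP_puzzle_part is an interactable puzzle piece that the player can pick up.
; On BeginPlay it caches the player pawn as BP_Player.
; When aimed at, it sets the player's focus enum; on interaction it flags the player as holding an object, records the object type enum, and destroys itself.
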(event EventAimed
  (Variables|/Game/Game/Character/Blueprint/BP_Player.BP_Player_C|SetEnum%20Focus%20REF (Variables|REF|GetPlayer%20REF) "NewEnumerator0"))

(event EventBeginPlay
  (bind _asbp_player (Utilities|Casting|CastToBP_Player (Game|Player|GetPlayerPawn 0)))
  (Variables|REF|SetPlayer%20REF _asbp_player))

(event EventInteract
  (bind _player_ref (Variables|REF|GetPlayer%20REF))
  (Variables|/Game/Game/Character/Blueprint/BP_Player.BP_Player_C|SetGot%20Object _player_ref true)
  (Variables|/Game/Game/Character/Blueprint/BP_Player.BP_Player_C|SetEnum%20Object%20REF _player_ref "NewEnumerator0")
  (Actor|DestroyActor))

(fn ConstructionScript)