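; BP_key_door is an interactable door that requires the player to hold a key, tracked by the Clé variable on BP_Player.
; It caches the player reference at BeginPlay.
; Aimed sets the player's focus enum, switching to a different state when the key is held.
; Interact with the key sets the player's object enum and destroys the door actor.
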(event EventAimed
  (Variables|/Game/Game/Character/Blueprint/BP_Player.BP_Player_C|SetEnum%20Focus%20REF (Variables|REF|GetPlayer%20REF) "NewEnumerator1")
  (if (== (Variables|/Game/Game/Character/Blueprint/BP_Player.BP_Player_C|Getclé (Variables|REF|GetPlayer%20REF)) 1)
    (Variables|/Game/Game/Character/Blueprint/BP_Player.BP_Player_C|SetEnum%20Focus%20REF (Variables|REF|GetPlayer%20REF) "NewEnumerator2")))

(event EventBeginPlay
  (bind _asbp_player (Utilities|Casting|CastToBP_Player (Game|Player|GetPlayerPawn 0)))
  (Variables|REF|SetPlayer%20REF _asbp_player))

(event EventInteract
  (bind _player_ref (Variables|REF|GetPlayer%20REF))
  (if (== (Variables|/Game/Game/Character/Blueprint/BP_Player.BP_Player_C|Getclé _player_ref) 1)
    (Variables|/Game/Game/Character/Blueprint/BP_Player.BP_Player_C|SetEnum%20Object%20REF _player_ref "NewEnumerator4")
    (Actor|DestroyActor)))

(fn ConstructionScript)