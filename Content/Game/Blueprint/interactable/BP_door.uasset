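; BP_door is an interactable door actor that is removed from the world when the player interacts with it.
; It caches the BP_Player pawn on BeginPlay, and its Aimed event writes that player's EnumFocusREF focus state.
; The branches in Interact and Aimed are fixed to true, so interaction always destroys the door and aiming always overwrites the first focus value with the second.
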(event EventAimed
  (Variables|/Game/Game/Character/Blueprint/BP_Player.BP_Player_C|SetEnum%20Focus%20REF (Variables|REF|GetPlayer%20REF) "NewEnumerator1")
  (if true
    (Variables|/Game/Game/Character/Blueprint/BP_Player.BP_Player_C|SetEnum%20Focus%20REF (Variables|REF|GetPlayer%20REF) "NewEnumerator2")))

(event EventBeginPlay
  (bind _asbp_player (Utilities|Casting|CastToBP_Player (Game|Player|GetPlayerPawn 0)))
  (Variables|REF|SetPlayer%20REF _asbp_player))

(event EventInteract
  (if true
    (Actor|DestroyActor)))

(fn ConstructionScript)